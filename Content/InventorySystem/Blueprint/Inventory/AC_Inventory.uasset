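; AC_Inventory is an inventory component that stores multi-tile items in a fixed grid, backed by a flat ItemArray sized from columns and rows.
; TryAddItem scans for the first area that fits the item's dimensions, retrying once rotated, then AddItemAt writes the item into every covered cell.
; RemoveItem clears matching cells, while GetAllItems maps each unique item to its top-left tile.
; Edits set IsDirty, which Tick turns into an OnInventoryChanged notification.
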(event `self.ReceiveBeginPlay`
  (`|ExecutionSequence`
    (:`then_0`
      ; SetGridToItemArray
      ;
      ; Initialise la taille de l’inventaire à la création du jeu ou de l’objet (Begin Play).
      ;
      ; 📥 Variables utilisées :
      ;
      ; - Nb Columns (Integer) : Nombre de colonnes de la grille.
      ; - Nb Rows (Integer) : Nombre de lignes de la grille.
      ; - ItemArray (Array of BP_ItemObject) : Tableau représentant l’état de chaque case de l’inventaire (vide ou occupée).
      ;
      ; 🧠 Utilité :
      ; - Cette étape est essentielle pour garantir que l’inventaire est prêt à être utilisé dès le départ.
      ; - Sans cette initialisation, les fonctions de placement, recherche ou affichage des objets dans l’inventaire n’auraient pas de base cohérente sur laquelle travailler.
      (`KismetArrayLibrary.Array_Resize` (`self.ItemArray`) (* (`self.NbColumns`) (`self.NbRows`))))))

(event `self.ReceiveTick`
  (params (DeltaSeconds :type "Float (single-precision)"))
  (`|ExecutionSequence`
    (:`then_0`
      ; Vérification du changement d'inventaire
      ;
      ; Ce script s’exécute à chaque frame et vérifie si l’inventaire a été modifié.
      ; S’il y a eu un changement, il déclenche un événement de mise à jour pour synchroniser l’affichage ou d'autres systèmes.
      ;
      ; 📥 Variables utilisées :
      ; - Is Dirty (bool) : Flag qui indique si un changement a été effectué dans l’inventaire (ajout, suppression, etc.).
      ; - Call OnInventoryChanged : Événement ou dispatcher qui notifie les systèmes liés à l’inventaire (comme l’UI) qu’une mise à jour est nécessaire.
      ;
      ; 🧠 Utilité :
      ; - Cela permet d’éviter les mises à jour inutiles :
      ; - On ne rafraîchit l’inventaire que si un changement a eu lieu, ce qui améliore les performances et évite des appels superflus.
      (if (`self.IsDirty`)
        (set `self.IsDirty` false)
        ;; Pas trop sur
        (`self.OnInventoryChanged` self)))))

(fn `AddItemAt`
  (params (ItemObject :type "/Game/InventorySystem/Blueprint/Items/BP_ItemObject Object Reference") (TopLeftIndex :type Integer))
  (bind _tile (`self.ForEachIndex` ItemObject TopLeftIndex)
    (:`LoopBody`
      (`KismetArrayLibrary.Array_Set` (`self.ItemArray`) (`self.TileToIndex` _tile) (`local.ItemObject`)))
    (:`Completed`
      (set `self.IsDirty` true))))

(fn `GetAllItems`
  (returns (AllItems :type "Map of /Game/InventorySystem/Blueprint/Items/BP_ItemObject Object Reference to /Game/InventorySystem/Blueprint/Items/S_Tile Structure"))
  (locals (`CurrentItemObject(Local)` :type "/Game/InventorySystem/Blueprint/Items/BP_ItemObject Object Reference") (`AllItems(Local)` :type "Map of /Game/InventorySystem/Blueprint/Items/BP_ItemObject Object Reference to /Game/InventorySystem/Blueprint/Items/S_Tile Structure"))
  (for (_array_element _array_index) (`self.ItemArray`)
    (bind _output_get (set `local.CurrentItemObject(Local)` _array_element))
    (`/Engine/EditorBlueprintResources/StandardMacros.IsValid` _output_get
      (:`Is Valid`
        (if (not (`BlueprintMapLibrary.Map_Contains` (`local.AllItems(Local)`) _array_element))
          (`BlueprintMapLibrary.Map_Add` (`local.AllItems(Local)`) (`local.CurrentItemObject(Local)`) (`self.IndexToTile` _array_index))))))
  (return (`local.AllItems(Local)`)))

(fn `GetItemAtIndex`
  (params (Index :type Integer))
  (returns (Valid :type Boolean) (ItemObject :type "/Game/InventorySystem/Blueprint/Items/BP_ItemObject Object Reference"))
  (if (`KismetArrayLibrary.Array_IsValidIndex` (`self.ItemArray`))
    (return true (`|GetArrayItem` (`self.ItemArray`) (`local.Index`)))
    (else
      (return false null))))

(fn `GetNumSlot`
  (returns (Return :type Integer))
  (return (* (`self.NbRows`) (`self.NbColumns`))))

(fn `IndexToTile`
  (params (Index :type Integer))
  (returns (Tile :type "/Game/InventorySystem/Blueprint/Items/S_Tile Structure"))
  (return (make `/Game/InventorySystem/Blueprint/Items/S_Tile` (mod Index (`self.NbColumns`)) (/ Index (`self.NbColumns`)))))

(fn `IsRoomAvailable`
  (params (ItemObject :type "/Game/InventorySystem/Blueprint/Items/BP_ItemObject Object Reference") (TopLeftIndex :type Integer))
  (returns (Success :type Boolean))
  (`|ExecutionSequence`
    (:`then_0`
      (bind _tile (`self.ForEachIndex` (`local.ItemObject`) (`local.TopLeftIndex`))
        (:`LoopBody`
          (`self.IsTileValid` _tile
            (:`true`
              (bind (_valid _itemobject) (`self.GetItemAtIndex` (`self.TileToIndex` _tile)))
              (if _valid
                (if (`KismetSystemLibrary.IsValid` _itemobject)
                  (return false))
                (else
                  (return false))))
            (:`false`
              (return false))))))
    (:`then_1`
      (return true))))

(fn `RemoveItem`
  (params (ItemObject :type "/Game/InventorySystem/Blueprint/Items/BP_ItemObject Object Reference"))
  (`/Engine/EditorBlueprintResources/StandardMacros.IsValid` ItemObject
    (:`Is Valid`
      (for (_array_element _array_index) (`self.ItemArray`)
        (if (== _array_element (`local.ItemObject`))
          (`KismetArrayLibrary.Array_Set` (`self.ItemArray`) _array_index)
          (set `self.IsDirty` true))))))

(fn `TileToIndex`
  (params (Tile :type "/Game/InventorySystem/Blueprint/Items/S_Tile Structure"))
  (returns (Index :type Integer))
  (bind (_x _y) (break `/Game/InventorySystem/Blueprint/Items/S_Tile` Tile))
  (return (+ _x (* _y (`self.NbColumns`)))))

(fn `TryAddItem`
  (params (ItemObject :type "/Game/InventorySystem/Blueprint/Items/BP_ItemObject Object Reference"))
  (returns (Success :type Boolean))
  (`/Engine/EditorBlueprintResources/StandardMacros.IsValid` ItemObject
    (:`Is Valid`
      (for (_ _array_index) (`self.ItemArray`) :!label _label
        (bind _success (`self.IsRoomAvailable` (`local.ItemObject`) _array_index))
        (if _success
          (`self.AddItemAt` (`local.ItemObject`) _array_index)
          (return true)))
      (`|ExecutionSequence`
        (:`then_0`
          (`/Engine/EditorBlueprintResources/StandardMacros.DoOnce` false
            (:`Completed`
              (`/Game/InventorySystem/Blueprint/Items/BP_ItemObject.Rotate` (`local.ItemObject`))
              (goto _label))))
        (:`then_1`
          (`/Game/InventorySystem/Blueprint/Items/BP_ItemObject.Rotate` (`local.ItemObject`))
          (return false))))
    (:`Is Not Valid`
      (`KismetSystemLibrary.PrintString` "Error:Item is not valid:AC_Inventory>TryAddItem "))))